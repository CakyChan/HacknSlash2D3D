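; BP_Character is a sprite-based character with two-axis movement, health and a floating nameplate.
; Forward and Shift inputs drive world X and Y movement, with the sprite flipped 180 degrees to face the X direction unless attacking.
; Capsule hits from another BP_Character subtract health.
; Tick reapplies facing when X velocity is zero and passes itself to the nameplate widget, showing it only when health differs from maximum.
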(event OnComponentHit(CapsuleComponent)
  (params (HitComponent :type Primitive%20Component%20Object%20Reference) (OtherActor :type Actor%20Object%20Reference) (OtherComp :type Primitive%20Component%20Object%20Reference) (NormalImpulse :type Vector :default "0, 0, 0") (Hit :type Hit%20Result%20Structure%20%28by%20ref%29))
  (Utilities|Casting|CastToBP_Character OtherActor)
  (Variables|Default|SetHp (- (Variables|Default|GetHp) 1)))

(event EventBeginPlay
  (Variables|Default|SetHp 100)
  (Variables|Default|SetMaxHp 100)
  (Variables|Default|SetisAttacking false))

(event EventTick
  (params (DeltaSeconds :type Float%20%28single-precision%29))
  (CallFunction|DisplayNameplate)
  (Math|Float|CompareFloat (.x (Variables|/Script/Engine.MovementComponent|GetVelocity (Variables|Character|GetCharacterMovement))) 0.0
    (:==
      (if (not (Variables|Default|GetisAttacking))
        (CallFunction|RotateSprite (Variables|Default|Getmoveright?))))))

(event Input|AxisEvents|InputAxisForward
  (params (AxisValue :type Float%20%28single-precision%29))
  (if (> AxisValue 0.0)
    (Variables|Default|Setmoveright? true)
    (elif (< AxisValue 0.0)
      (Variables|Default|Setmoveright? false)))
  (if (Variables|Default|GetisAttacking)
    _
    (else
      (CallFunction|RotateSprite (Variables|Default|Getmoveright?))))
  (Pawn|Input|AddMovementInput "1.000000,0.000000,0.000000" AxisValue false))

(event Input|AxisEvents|InputAxisShift
  (params (AxisValue :type Float%20%28single-precision%29))
  (Pawn|Input|AddMovementInput "0.000000,1.000000,0.000000" AxisValue false))

(fn ConstructionScript)

(fn DisplayNameplate
  (bind _asbp_character_nameplate (Utilities|Casting|CastToBP_Character_Nameplate (UserInterface|GetUserWidgetObject (Variables|Default|Getnameplate))))
  (bind _output_get (Variables|/Game/Content/Blueprints/Character/BP_Character_Nameplate.BP_Character_Nameplate_C|SetCharacter _asbp_character_nameplate self))
  (Rendering|SetVisibility (Variables|Default|Getnameplate) (!= (Variables|BP_Character_C|GetHp _output_get) (Variables|BP_Character_C|GetMaxHp _output_get)) false))

(fn RotateSprite
  (params (moveRight? :type Boolean))
  (Variables|Default|Setmoveright? moveRight?)
  (if moveRight?
    (Transformation|SetRelativeRotation (Variables|Default|GetSprite) "0, 0, 0" false false)
    (else
      (Transformation|SetRelativeRotation (Variables|Default|GetSprite) "0.000000,180.000000,0.000000" false false)))
  (return))