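; BP_Skeleton is the skeleton enemy character, which sets its name and health on BeginPlay.
; Tick polls DidHpChanged and IsCharacterDead, then drives the animation state machine through JumpToNode to play either the hit or the dying reaction.
; On death it disables capsule collision and destroys the actor after a short delay.
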(event EventBeginPlay
  (|CallParentFunction)
  (Variables|Default|SetName "Skeleton")
  (Variables|Default|SetHp 100)
  (Variables|Default|SetMaxHp 100))

(event Collision|EventActorBeginOverlap
  (params (OtherActor :type Actor%20Object%20Reference))
  (|CallParentFunction OtherActor) ; This node is disabled and will not be called.\nDrag off pins to build functionality.
)

(event EventTick
  (params (DeltaSeconds :type Float%20%28single-precision%29))
  (bind _animationcomponent (Variables|Default|GetAnimationComponent))
  (bind _animinstance (Variables|/Script/PaperZD.PaperZDAnimationComponent|GetAnimInstance _animationcomponent))
  (|CallParentFunction DeltaSeconds)
  (bind _hpchanged_ (CallFunction|DidHpChanged?))
  (if _hpchanged_
    (bind _characterdead_ (CallFunction|IsCharacterDead?))
    (if _characterdead_
      (Class|PaperZDAnimInstance|JumptoNode _animinstance "OnDying" "None")
      (Collision|SetCollisionEnabled (Variables|Default|GetCapsuleComponent) "NoCollision")
      (Utilities|FlowControl|Delay 1.5)
      (Actor|DestroyActor)
      (else
        (Class|PaperZDAnimInstance|JumptoNode _animinstance "OnHit" "None")))))

(fn ConstructionScript
  (|CallParentFunction))