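; BP_FireballExplosion is the short-lived explosion effect actor for the hero's fireball spell.
; On BeginPlay it orients its PaperFlipbook by comparing the actor's world X, as a percentage of viewport width, against the halfway mark, rotating the sprite 180 degrees at or below it.
; It then destroys itself after a brief delay, with no overlap or tick logic.
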(event EventBeginPlay
  (if (> (/ (* (.X (Class|KismetMathLibrary|BreakVector3f (Transformation|GetActorLocation))) 1e+02) (.X (Math|Vector2D|BreakVector2D (Viewport|GetViewportSize)))) 5e+01)
    (Transformation|SetRelativeRotation (Variables|Default|GetPaperFlipbook) "0, 0, 0" false false)
    (else
      (Transformation|SetRelativeRotation (Variables|Default|GetPaperFlipbook) "0.000000,180.000000,0.000000" false false)))
  (Utilities|FlowControl|Delay 0.3)
  (Actor|DestroyActor))

(event Collision|EventActorBeginOverlap
  (params (OtherActor :type Actor%20Object%20Reference)))

(event EventTick
  (params (DeltaSeconds :type Float%20%28single-precision%29)))

(fn ConstructionScript)