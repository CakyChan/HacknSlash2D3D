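; BP_Hero is the sprite-based player hero, initializing health and spell state, showing the mouse cursor and handling attack and spell input.
; Spell1 flips the sprite by cursor screen side and launches a fireball toward the traced cursor point, briefly disabling its collision.
; Spell2 is a timed haste buff raising GcdMultiplier, which shortens Spell1's cooldown.
; Attack only jumps the animation state machine to its attack node.
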(event EventBeginPlay
  (Variables|/Script/Engine.PlayerController|SetbShowMouseCursor (Game|GetPlayerController 0) true)
  (Variables|Default|SetName "Hero")
  (Variables|Default|SetHp 100)
  (Variables|Default|SetMaxHp 100)
  (Variables|Default|SetisAttacking false)
  (Variables|Default|SetgcdMultiplier 1.0)
  (Variables|Default|SetcanSpell1? true)
  (Variables|Default|SetcdSpell1 0.3)
  (Variables|Default|SetcanSpell2? true))

(event Collision|EventActorBeginOverlap
  (params (OtherActor :type Actor%20Object%20Reference)))

(event EventTick
  (params (DeltaSeconds :type Float%20%28single-precision%29)))

(event Input|ActionEvents|InputActionSpell1
  (params (Key :type Key%20Structure :default "None"))
  (bind _returnvalue (Game|GetPlayerController 0))
  (bind _returnvalue_2 (Transformation|GetActorLocation))
  (bind _hitresult (Game|Player|GetHitResultUnderCursorbyChannel _returnvalue "TraceTypeQuery2" true))
  (bind _impactpoint (Collision|BreakHitResult _hitresult))
  (bind _returnvalue_3 (Math|Rotator|FindLookatRotation _returnvalue_2 _impactpoint))
  (bind (_x _y _z) (Math|Rotator|BreakRotIntoAxes _returnvalue_3))
  (:Pressed
    (if (and (Variables|Default|GetcanSpell1?) (not (Variables|Default|GetisAttacking)))
      (Class|PaperZDAnimInstance|JumptoNode (Variables|/Script/PaperZD.PaperZDAnimationComponent|GetAnimInstance (Variables|Default|GetAnimationComponent)) "Spellbind" "None")
      (bind _returnvalue_4 (Class|WidgetLayoutLibrary|GetMousePositiononViewport))
      (Variables|Default|SetisAttacking true)
      (CallFunction|RotateSprite (> (/ (* (.X (Math|Vector2D|BreakVector2D _returnvalue_4)) 1e+02 (Class|WidgetLayoutLibrary|GetViewportScale)) (.X (Math|Vector2D|BreakVector2D (Viewport|GetViewportSize)))) 5e+01))
      (bind _returnvalue_5 (Game|SpawnActorfromClass "/Game/Content/Blueprints/Character/Hero/Spells/BP_Fireball.BP_Fireball_C" (Math|Transform|MakeTransform _returnvalue_2 (Math|Rotator|MakeRotationfromAxes (Math|Vector|MakeVector (.x _x) (.y _x) 0.0) _y _z) "0.200000,0.200000,0.200000") "AlwaysSpawn" self 0))
      (Variables|Default|SetcanSpell1? false)
      (Collision|SetCollisionEnabled (Variables|/Game/Content/Blueprints/Character/Hero/Spells/BP_Fireball.BP_Fireball_C|GetSphere _returnvalue_5) "NoCollision")
      (Utilities|FlowControl|Delay 0.1)
      (Collision|SetCollisionEnabled (Variables|/Game/Content/Blueprints/Character/Hero/Spells/BP_Fireball.BP_Fireball_C|GetSphere _returnvalue_5) "QueryAndPhysics")
      (Utilities|FlowControl|Delay (Math|Float|SafeDivide (Variables|Default|GetcdSpell1) (Variables|Default|GetgcdMultiplier)))
      (Variables|Default|SetcanSpell1? true)
      (Variables|Default|SetisAttacking false))))

(event Input|ActionEvents|InputActionAttack
  (params (Key :type Key%20Structure :default "None"))
  (:Pressed
    (Class|PaperZDAnimInstance|JumptoNode (Variables|/Script/PaperZD.PaperZDAnimationComponent|GetAnimInstance (Variables|Default|GetAnimationComponent)) "Attack" "None")))

(event Input|ActionEvents|InputActionSpell2
  (params (Key :type Key%20Structure :default "None"))
  (:Pressed
    (if (Variables|Default|GetcanSpell2?)
      (Variables|Default|SetcanSpell2? false)
      (Variables|Default|SetgcdMultiplier 3.0)
      (Utilities|FlowControl|Delay 2e+01)
      (Variables|Default|SetgcdMultiplier 1.0)
      (Variables|Default|SetcanSpell2? true))))

(fn ConstructionScript
  (|CallParentFunction))