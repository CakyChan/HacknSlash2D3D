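; AN_Attack is an animation notify in the Hero folder that performs a box overlap check for an attack, currently as a debug stub.
; With a valid owning instance, it queries actors in a box at the sequence render component's location, with no object types specified, and prints placeholder messages.
; Without one, it draws a debug box of the same extent, previewing the hit area.
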(event EventOnReceiveNotify
  (params (OwningInstance :type Paper%20ZD%20Anim%20Instance%20Object%20Reference))
  (bind _sequencerendercomponent (Variables|Default|GetSequenceRenderComponent))
  (bind _extent (Variables|Default|GetExtent))
  (bind _returnvalue (Transformation|GetWorldLocation _sequencerendercomponent))
  (Utilities|IsValid OwningInstance
    (:Is%20Valid
      (bind _outactors (Collision|BoxOverlapActors _returnvalue _extent (Utilities|Array|MakeArray) 0 :!class /Script/Engine.KismetSystemLibrary))
      (for _array_element _outactors
        (Development|PrintString "Hello"))
      (Development|PrintString "Hello"))
    (:Is%20Not%20Valid
      (Rendering|Debug|DrawDebugBox :Center _returnvalue :Extent _extent))))