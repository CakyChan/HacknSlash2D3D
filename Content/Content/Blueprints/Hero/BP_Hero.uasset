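; Player hero character with a PaperZD-animated sprite that moves, attacks, casts fireballs and tracks its health.
; Axis input moves it along world X and Y, with the sprite flipped to match the last X direction.
; Attack and Spell1 jump to animation nodes, and Spell1 also spawns BP_Fireball above the hero, oriented from a cursor-trace look-at.
; Capsule hits from BP_EnemyTest subtract health, with no death handling here.
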(event OnComponentHit(CapsuleComponent)
  (params (HitComponent :type Primitive%20Component%20Object%20Reference) (OtherActor :type Actor%20Object%20Reference) (OtherComp :type Primitive%20Component%20Object%20Reference) (NormalImpulse :type Vector :default "0, 0, 0") (Hit :type Hit%20Result%20Structure%20%28by%20ref%29))
  (Utilities|Casting|CastToBP_EnemyTest OtherActor)
  (Variables|Default|SetHero_Hp (- (Variables|Default|GetHero_Hp) 5)))

(event EventBeginPlay
  (Variables|Default|SetHero_Hp 100)
  (Variables|Default|SetHero_maxHp 100)
  (Variables|/Script/Engine.PlayerController|SetbShowMouseCursor (Game|GetPlayerController 0) true)
  (Variables|Default|SetHero_name "Hero"))

(event EventTick
  (params (DeltaSeconds :type Float%20%28single-precision%29))
  (Math|Float|CompareFloat (.x (Variables|/Script/Engine.MovementComponent|GetVelocity (Variables|Character|GetCharacterMovement))) 0.0
    (:==
      (if (Variables|Default|Getmoveright?)
        (Transformation|SetRelativeRotation (Variables|Default|GetSprite) "0, 0, 0" false false)
        (else
          (Transformation|SetRelativeRotation (Variables|Default|GetSprite) "0.000000,180.000000,0.000000" false false))))))

(event Input|ActionEvents|InputActionSpell1
  (params (Key :type Key%20Structure :default "None"))
  (bind _returnvalue (Game|GetPlayerController 0))
  (bind _returnvalue_2 (Transformation|GetActorLocation))
  (bind _hitresult (Game|Player|GetHitResultUnderCursorbyChannel _returnvalue "TraceTypeQuery1" true))
  (bind _location (Collision|BreakHitResult _hitresult))
  (bind _returnvalue_3 (Math|Rotator|FindLookatRotation _returnvalue_2 _location))
  (bind (_x _y) (Math|Rotator|BreakRotIntoAxes _returnvalue_3))
  (:Pressed
    (Class|PaperZDAnimInstance|JumptoNode (Variables|/Script/PaperZD.PaperZDAnimationComponent|GetAnimInstance (Variables|Default|GetAnimationComponent)) "Spellbind" "None")
    (Game|SpawnActorfromClass "/Game/Content/Blueprints/Hero/Spells/BP_Fireball.BP_Fireball_C" (Math|Transform|MakeTransform (+ _returnvalue_2 "0.000000,0.000000,100.000000") (Math|Rotator|MakeRotationfromAxes _x _y "0, 0, 0")) "AlwaysSpawn" 0 0)))

(event Input|ActionEvents|InputActionAttack
  (params (Key :type Key%20Structure :default "None"))
  (:Pressed
    (Class|PaperZDAnimInstance|JumptoNode (Variables|/Script/PaperZD.PaperZDAnimationComponent|GetAnimInstance (Variables|Default|GetAnimationComponent)) "Attack" "None")))

(event Input|AxisEvents|InputAxisForward
  (params (AxisValue :type Float%20%28single-precision%29))
  (if (> AxisValue 0.0)
    (Variables|Default|Setmoveright? true)
    (Transformation|SetRelativeRotation (Variables|Default|GetSprite) "0, 0, 0" false false)
    (elif (< AxisValue 0.0)
      (Variables|Default|Setmoveright? false)
      (Transformation|SetRelativeRotation (Variables|Default|GetSprite) "0.000000,180.000000,0.000000" false false)))
  (Pawn|Input|AddMovementInput "1.000000,0.000000,0.000000" AxisValue false))

(event Input|AxisEvents|InputAxisShift
  (params (AxisValue :type Float%20%28single-precision%29))
  (Pawn|Input|AddMovementInput "0.000000,1.000000,0.000000" AxisValue false))

(fn ConstructionScript)