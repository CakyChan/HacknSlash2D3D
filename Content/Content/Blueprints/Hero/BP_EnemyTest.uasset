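; BP_EnemyTest is an input-driven 2D sprite character that, despite its name, behaves like a player hero test pawn.
; Forward and Shift axes move it along world X and Y, while Attack jumps the animation instance to its Attack node.
; Forward input sets the Moveright facing flag and flips the sprite by rotation, which Tick reapplies whenever X velocity is zero.
; BeginPlay initializes hero health values, which the graph never uses afterward.
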(event EventBeginPlay
  (Variables|Default|SetHero_Hp 100)
  (Variables|Default|SetHero_maxHp 100))

(event Collision|EventActorBeginOverlap
  (params (OtherActor :type Actor%20Object%20Reference)))

(event EventTick
  (params (DeltaSeconds :type Float%20%28single-precision%29))
  (Math|Float|CompareFloat (.x (Variables|/Script/Engine.MovementComponent|GetVelocity (Variables|Character|GetCharacterMovement))) 0.0
    (:==
      (if (Variables|Default|Getmoveright?)
        (Transformation|SetRelativeRotation (Variables|Default|GetSprite) "0, 0, 0" false false)
        (else
          (Transformation|SetRelativeRotation (Variables|Default|GetSprite) "0.000000,180.000000,0.000000" false false))))))

(event Input|ActionEvents|InputActionAttack
  (params (Key :type Key%20Structure :default "None"))
  (:Pressed
    (Class|PaperZDAnimInstance|JumptoNode (Variables|/Script/PaperZD.PaperZDAnimationComponent|GetAnimInstance (Variables|Default|GetAnimationComponent)) "Attack" "None")))

(event Input|AxisEvents|InputAxisForward
  (params (AxisValue :type Float%20%28single-precision%29))
  (if (> AxisValue 0.0)
    (Variables|Default|Setmoveright? true)
    (Transformation|SetRelativeRotation (Variables|Default|GetSprite) "0, 0, 0" false false)
    (elif (< AxisValue 0.0)
      (Variables|Default|Setmoveright? false)
      (Transformation|SetRelativeRotation (Variables|Default|GetSprite) "0.000000,180.000000,0.000000" false false)))
  (Pawn|Input|AddMovementInput "1.000000,0.000000,0.000000" AxisValue false))

(event Input|AxisEvents|InputAxisShift
  (params (AxisValue :type Float%20%28single-precision%29))
  (Pawn|Input|AddMovementInput "0.000000,1.000000,0.000000" AxisValue false))

(fn ConstructionScript)